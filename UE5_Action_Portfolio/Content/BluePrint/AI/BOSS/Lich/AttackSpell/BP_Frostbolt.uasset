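; Frostbolt projectile, filed under the Lich boss's attack spells, that triggers a field system where it stops.
; It plays the frostbolt sound cue on BeginPlay.
; When projectile movement stops, it spawns an FS_MasterField at the impact point, destroys itself, then sets the field's activation type and triggers it.
; The field's delayed cleanup is sequenced after the bolt's own destruction.
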(event `self.ReceiveBeginPlay`
  (bind _audio (`self.Audio`))
  (`AudioComponent.SetSound` _audio "/Game/BluePrint/AI/BOSS/Lich/AttackSpell/Sound/Cue_Frostbolt.Cue_Frostbolt")
  (`AudioComponent.Play` _audio 0.0))

(event `self.ProjectileMovement.OnProjectileStop`
  (params (ImpactResult :type "HitResult Structure (by ref)"))
  (bind _returnvalue (`|SpawnActorFromClass` "/Engine/EditorResources/FieldNodes/FS_MasterField.FS_MasterField_C" (`KismetMathLibrary.MakeTransform` ImpactResult_Location) "AlwaysSpawn" "OverrideRootScale" null null))
  (`self.K2_DestroyActor`)
  (set `/Engine/EditorResources/FieldNodes/FS_MasterField.ActivationType` "NewEnumerator4" _returnvalue)
  (`/Engine/EditorResources/FieldNodes/FS_MasterField.CE_Trigger` _returnvalue)
  (`KismetSystemLibrary.Delay` 0.2)
  (`self.K2_DestroyActor` _returnvalue))

(fn `UserConstructionScript`)