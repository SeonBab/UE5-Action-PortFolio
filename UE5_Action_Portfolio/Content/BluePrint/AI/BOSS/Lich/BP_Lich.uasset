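; Lich boss Blueprint that drives the boss's phase visuals and its HUD info panel.
; Tick reads the Phase blackboard value every frame and swaps the mesh material among three phase variants.
; The BossInfo on event shows the panel through BP_GameUIHUD's main widget and fills in name, HP and max HP.
; The off event and Destroyed share one path that hides the panel.
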(event `self.ReceiveTick`
  (params (DeltaSeconds :type "Float (single-precision)"))
  (bind _returnvalue (`BlackboardComponent.GetValueAsInt` (`self.BlackboardComponent`) "Phase"))
  (if (== _returnvalue 1)
    (`PrimitiveComponent.SetMaterial` (`self.Mesh`) 0 "/Game/BluePrint/AI/BOSS/Lich/Materials/MI_Lich_1.MI_Lich_1")
    (elif (== _returnvalue 2)
      (`PrimitiveComponent.SetMaterial` (`self.Mesh`) 0 "/Game/BluePrint/AI/BOSS/Lich/Materials/MI_Lich_2.MI_Lich_2")
      (elif (== _returnvalue 3)
        (`PrimitiveComponent.SetMaterial` (`self.Mesh`) 0 "/Game/BluePrint/AI/BOSS/Lich/Materials/MI_Lich_3.MI_Lich_3")
        (else
          (`KismetSystemLibrary.PrintString` "PhaseOver"))))))

(event `self.BpEventCallBossInfoOn`
  (bind _asbp_game_uihud (cast `/Game/BluePrint/UI/BP_GameUIHUD` (`PlayerController.GetHUD` (`GameplayStatics.GetPlayerController` 0)))
    (:`then`
      (bind _returnvalue (`GameUIHUD.GetMainWidget` _asbp_game_uihud))
      (`|ExecutionSequence`
        (:`then_0`
          (`MainWidget.SetBossInfoOnOff` _returnvalue true))
        (:`then_1`
          (bind _aswbp_main_widget (cast `/Game/BluePrint/UI/WBP_MainWidget` _returnvalue)
            (:`then`
              (`|ExecutionSequence`
                (:`then_0`
                  (bind _returnvalue_2 (`self.GetDataName`)))
                (:`then_1`
                  (bind _returnvalue_3 (`self.GetHP`)))
                (:`then_2`
                  (bind _returnvalue_4 (`self.GetMaxHP`))
                  (`BossInfo.SetBossInfo` (`/Game/BluePrint/UI/WBP_MainWidget.WBP_BossInfo` _aswbp_main_widget) _returnvalue_2 _returnvalue_3 _returnvalue_4))))
            (:`CastFailed`
              (`KismetSystemLibrary.PrintString` "CastFailed_MainWidget"))))))
    (:`CastFailed`
      (`KismetSystemLibrary.PrintString` "CastFailed_GameUIHUD"))))

(event `self.ReceiveDestroyed`
  (bind _asbp_game_uihud (cast `/Game/BluePrint/UI/BP_GameUIHUD` (`PlayerController.GetHUD` (`GameplayStatics.GetPlayerController` 0)) :!label _label)
    (:`then`
      (bind _returnvalue (`GameUIHUD.GetMainWidget` _asbp_game_uihud))
      (`MainWidget.SetBossInfoOnOff` _returnvalue false))
    (:`CastFailed`
      (`KismetSystemLibrary.PrintString` "CastFailed_GameUIHUD"))))

(event `self.BpEventCallBossInfoOff`
  (goto _label))

(fn `UserConstructionScript`)