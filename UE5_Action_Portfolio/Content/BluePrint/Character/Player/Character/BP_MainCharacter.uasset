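; Player character Blueprint that connects Enhanced Input to combat, movement, camera and weapon-switch actions, and drives the main HUD widget.
; BeginPlay assigns FOV, spring-arm and aim-screen curves, shows the HP bar and weapon slot, and adds the input mapping context.
; Input events forward to character functions, zeroing held axes on release.
; HP updates on its event, while the weapon icon refreshes both every Tick and on slot change.
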(event `self.ReceiveBeginPlay`
  (`|ExecutionSequence`
    (:`then_0`
      (`|ExecutionSequence`
        (:`then_0`
          (set `self.FOVCurveFloat` "/Game/BluePrint/Character/Player/Character/CB_ChangeFOV.CB_ChangeFOV"))
        (:`then_1`
          (set `self.CameraSpringArmVector` "/Game/BluePrint/Character/Player/Character/CB_ChangeArm.CB_ChangeArm"))
        (:`then_2`
          (set `self.AimScreenCurveFloat` "/Game/BluePrint/Character/Player/Character/CB_ChangeAimScreen.CB_ChangeAimScreen"))))
    (:`then_1`
      (bind _asbp_game_uihud (cast `/Game/BluePrint/UI/BP_GameUIHUD` (`PlayerController.GetHUD` (`GameplayStatics.GetPlayerController` 0)))
        (:`then`
          (bind _returnvalue (`GameUIHUD.GetMainWidget` _asbp_game_uihud))
          (bind _aswbp_main_widget (cast `/Game/BluePrint/UI/WBP_MainWidget` _returnvalue)
            (:`then`
              (`|ExecutionSequence`
                (:`then_0`
                  (`MainWidget.SetMainCharHpBarOnOff` _aswbp_main_widget true))
                (:`then_1`
                  (`MainWidget.SetWeaponSlotOnOff` _aswbp_main_widget true))))
            (:`CastFailed`
              (`KismetSystemLibrary.PrintString` "CastFailed_MainWidget"))))
        (:`CastFailed`
          (`KismetSystemLibrary.PrintString` "CastFailed_GameUIHUD"))))
    (:`then_2`
      (`EnhancedInputSubsystemInterface.AddMappingContext` (pcsubsystem `EnhancedInputLocalPlayerSubsystem` (`GameplayStatics.GetPlayerController` 0)) "/Game/BluePrint/Character/Player/Input/EI_PlayerInput.EI_PlayerInput" 0 (struct)))))

(event `self.BpEventCallHPBar`
  (bind _asbp_game_uihud (cast `/Game/BluePrint/UI/BP_GameUIHUD` (`PlayerController.GetHUD` (`GameplayStatics.GetPlayerController` 0)))
    (:`then`
      (bind _returnvalue (`GameUIHUD.GetMainWidget` _asbp_game_uihud))
      (bind _aswbp_main_widget (cast `/Game/BluePrint/UI/WBP_MainWidget` _returnvalue)
        (:`then`
          (`|ExecutionSequence`
            (:`then_0`
              (bind _returnvalue_2 (`self.GetHP`)))
            (:`then_1`
              (bind _returnvalue_3 (`self.GetMaxHP`))
              (`HealthBar.SetHPInfo` (`/Game/BluePrint/UI/WBP_MainWidget.WBP_HP` _aswbp_main_widget) _returnvalue_2 _returnvalue_3))))
        (:`CastFailed`
          (`KismetSystemLibrary.PrintString` "CastFailed_MainWidget"))))
    (:`CastFailed`
      (`KismetSystemLibrary.PrintString` "CastFailed_GameUIHUD"))))

(event `self.ReceiveTick`
  (params (DeltaSeconds :type "Float (single-precision)"))
  (bind _asbp_game_uihud (cast `/Game/BluePrint/UI/BP_GameUIHUD` (`PlayerController.GetHUD` (`GameplayStatics.GetPlayerController` 0)) :!label _label)
    (:`then`
      (bind _returnvalue (`GameUIHUD.GetMainWidget` _asbp_game_uihud))
      (bind _aswbp_main_widget (cast `/Game/BluePrint/UI/WBP_MainWidget` _returnvalue)
        (:`then`
          (bind _returnvalue_2 (`self.GetWeaponComponent`))
          (bind _returnvalue_3 (`WeaponComponent.GetWeaponType` _returnvalue_2))
          (`WeaponSlot.SetWpSlotIcon` (`/Game/BluePrint/UI/WBP_MainWidget.WBP_WeaponSlot` _aswbp_main_widget) _returnvalue_3))
        (:`CastFailed`
          (`KismetSystemLibrary.PrintString` "CastFailed_MainWidget"))))
    (:`CastFailed`
      (`KismetSystemLibrary.PrintString` "CastFailed_GameUIHUD"))))

(event `self.BpEventChangeWpSlot`
  (goto _label))

(event `EnhancedInput|/Game/BluePrint/Character/Player/Input/EI_PlayerMoveFB`
  (params (ActionValue :type "Float (double-precision)") (ElapsedSeconds :type "Float (double-precision)") (TriggeredSeconds :type "Float (double-precision)") (InputAction :type "InputAction Object Reference" :default "/Game/BluePrint/Character/Player/Input/EI_PlayerMoveFB.EI_PlayerMoveFB"))
  (:`Triggered`
    (`self.MoveForward` ActionValue))
  (:`Canceled`
    (`self.MoveForward` 0.0 :!label _label))
  (:`Completed`
    (goto _label)))

(event `EnhancedInput|/Game/BluePrint/Character/Player/Input/EI_PlayerLockOn`
  (params (ActionValue :type Boolean) (ElapsedSeconds :type "Float (double-precision)") (TriggeredSeconds :type "Float (double-precision)") (InputAction :type "InputAction Object Reference" :default "/Game/BluePrint/Character/Player/Input/EI_PlayerLockOn.EI_PlayerLockOn"))
  (:`Started`
    (`self.LockOnTarget`)))

(event `EnhancedInput|/Game/BluePrint/Character/Player/Input/EI_PlayerMouseL`
  (params (ActionValue :type Boolean) (ElapsedSeconds :type "Float (double-precision)") (TriggeredSeconds :type "Float (double-precision)") (InputAction :type "InputAction Object Reference" :default "/Game/BluePrint/Character/Player/Input/EI_PlayerMouseL.EI_PlayerMouseL"))
  (:`Started`
    (`self.Attack`)))

(event `EnhancedInput|/Game/BluePrint/Character/Player/Input/EI_PlayerUnArmedChange`
  (params (ActionValue :type Boolean) (ElapsedSeconds :type "Float (double-precision)") (TriggeredSeconds :type "Float (double-precision)") (InputAction :type "InputAction Object Reference" :default "/Game/BluePrint/Character/Player/Input/EI_PlayerUnArmedChange.EI_PlayerUnArmedChange"))
  (:`Started`
    (`self.ChangeUnArmed`)))

(event `EnhancedInput|/Game/BluePrint/Character/Player/Input/EI_PlayerMouseR`
  (params (ActionValue :type "Float (double-precision)") (ElapsedSeconds :type "Float (double-precision)") (TriggeredSeconds :type "Float (double-precision)") (InputAction :type "InputAction Object Reference" :default "/Game/BluePrint/Character/Player/Input/EI_PlayerMouseR.EI_PlayerMouseR"))
  (:`Triggered`
    (`self.AimorBlock` ActionValue))
  (:`Canceled`
    (`self.AimorBlock` 0.0 :!label _label_2))
  (:`Completed`
    (goto _label_2)))

(event `EnhancedInput|/Game/BluePrint/Character/Player/Input/EI_PlayerBowChange`
  (params (ActionValue :type Boolean) (ElapsedSeconds :type "Float (double-precision)") (TriggeredSeconds :type "Float (double-precision)") (InputAction :type "InputAction Object Reference" :default "/Game/BluePrint/Character/Player/Input/EI_PlayerBowChange.EI_PlayerBowChange"))
  (:`Started`
    (`self.ChangeBow`)))

(event `EnhancedInput|/Game/BluePrint/Character/Player/Input/EI_PlayerMoveLR`
  (params (ActionValue :type "Float (double-precision)") (ElapsedSeconds :type "Float (double-precision)") (TriggeredSeconds :type "Float (double-precision)") (InputAction :type "InputAction Object Reference" :default "/Game/BluePrint/Character/Player/Input/EI_PlayerMoveLR.EI_PlayerMoveLR"))
  (:`Triggered`
    (`self.MoveRight` ActionValue))
  (:`Canceled`
    (`self.MoveRight` 0.0 :!label _label_3))
  (:`Completed`
    (goto _label_3)))

(event `EnhancedInput|/Game/BluePrint/Character/Player/Input/EI_PlayerMouseTurn`
  (params (ActionValue :type "Vector2D Structure") (ElapsedSeconds :type "Float (double-precision)") (TriggeredSeconds :type "Float (double-precision)") (InputAction :type "InputAction Object Reference" :default "/Game/BluePrint/Character/Player/Input/EI_PlayerMouseTurn.EI_PlayerMouseTurn"))
  (:`Triggered`
    (`self.AddControllerYawInput` (* ActionValue_X 0.5))
    (`self.AddControllerPitchInput` (* ActionValue_Y -0.5))))

(event `EnhancedInput|/Game/BluePrint/Character/Player/Input/EI_PlayerWheelUD`
  (params (ActionValue :type "Float (double-precision)") (ElapsedSeconds :type "Float (double-precision)") (TriggeredSeconds :type "Float (double-precision)") (InputAction :type "InputAction Object Reference" :default "/Game/BluePrint/Character/Player/Input/EI_PlayerWheelUD.EI_PlayerWheelUD"))
  (:`Triggered`
    (if (== ActionValue 1.0)
      (`self.ZoomIn`)
      (elif (== ActionValue -1.0)
        (`self.ZoomOut`)))))

(event `EnhancedInput|/Game/BluePrint/Character/Player/Input/EI_PlayerParry`
  (params (ActionValue :type Boolean) (ElapsedSeconds :type "Float (double-precision)") (TriggeredSeconds :type "Float (double-precision)") (InputAction :type "InputAction Object Reference" :default "/Game/BluePrint/Character/Player/Input/EI_PlayerParry.EI_PlayerParry"))
  (:`Started`
    (`self.Parry`)))

(event `EnhancedInput|/Game/BluePrint/Character/Player/Input/EI_PlayerSwordChange`
  (params (ActionValue :type Boolean) (ElapsedSeconds :type "Float (double-precision)") (TriggeredSeconds :type "Float (double-precision)") (InputAction :type "InputAction Object Reference" :default "/Game/BluePrint/Character/Player/Input/EI_PlayerSwordChange.EI_PlayerSwordChange"))
  (:`Started`
    (`self.ChangeSwordAndSheiled`)))

(event `EnhancedInput|/Game/BluePrint/Character/Player/Input/EI_PlayerRollorRun`
  (params (ActionValue :type "Float (double-precision)") (ElapsedSeconds :type "Float (double-precision)") (TriggeredSeconds :type "Float (double-precision)") (InputAction :type "InputAction Object Reference" :default "/Game/BluePrint/Character/Player/Input/EI_PlayerRollorRun.EI_PlayerRollorRun"))
  (:`Triggered`
    (`self.RollorRun` ActionValue))
  (:`Canceled`
    (`self.RollorRun` 0.0 :!label _label_4))
  (:`Completed`
    (goto _label_4)))

(event `EnhancedInput|/Game/BluePrint/Character/Player/Input/EI_PalyerJump`
  (params (ActionValue :type Boolean) (ElapsedSeconds :type "Float (double-precision)") (TriggeredSeconds :type "Float (double-precision)") (InputAction :type "InputAction Object Reference" :default "/Game/BluePrint/Character/Player/Input/EI_PalyerJump.EI_PalyerJump"))
  (:`Started`
    (`self.JumpAction`)))

(fn `UserConstructionScript`)