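; BP_Paladin is a Paladin monster Blueprint that shows an overhead health display.
; Each Tick it rotates the Widget component toward the player camera, billboard style.
; It also casts the widget to WBP_OverHeadInfo and sets the HPBar's horizontal render scale to the HP/MaxHP ratio by polling, printing a debug string if the cast fails.
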(event `self.ReceiveTick`
  (params (DeltaSeconds :type "Float (single-precision)"))
  (bind _widget (`self.Widget`))
  (`|ExecutionSequence`
    (:`then_0`
      (`SceneComponent.K2_SetWorldRotation` _widget (`KismetMathLibrary.FindLookAtRotation` (`SceneComponent.K2_GetComponentLocation` _widget) (`SceneComponent.K2_GetComponentLocation` (`PlayerCameraManager.TransformComponent` (`GameplayStatics.GetPlayerCameraManager` 0)))) false false))
    (:`then_1`
      (bind _aswbp_over_head_info (cast `/Game/BluePrint/UI/WBP_OverHeadInfo` (`WidgetComponent.GetWidget` (`self.Widget`)))
        (:`then`
          (`|ExecutionSequence`
            (:`then_0`
              (bind _returnvalue (`self.GetHP`)))
            (:`then_1`
              (bind _returnvalue_2 (`self.GetMaxHP`)))
            (:`then_2`
              (`Widget.SetRenderScale` (`/Game/BluePrint/UI/WBP_OverHeadInfo.HPBar` _aswbp_over_head_info) (`KismetMathLibrary.MakeVector2D` (/ _returnvalue _returnvalue_2) 1.0)))))
        (:`CastFailed`
          (`KismetSystemLibrary.PrintString` "CastFailed_OverHeadInfo"))))))

(fn `UserConstructionScript`)